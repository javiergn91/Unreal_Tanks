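; Player-controllable tank Blueprint that sets up the tank's components and routes input for driving, camera orbit and firing.
; On BeginPlay it registers the barrel and turret and hands both tracks to the TankMovement component.
; Driving accepts either direct per-track throttle or forward/right intents through TankMovement.
; Aim axes rotate the azimuth gimbal and spring arm at frame-rate-independent speed, and the Fire action calls Fire.
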(event `self.ReceiveBeginPlay`
  (`self.SetBarrel` (`self.TankBarrel`))
  (`self.SetTurret` (`self.TankTurret`))
  (`TankMovement.Initialise` (`self.TankMovement`) (`self.LeftTrack`) (`self.RightTrack`)))

(event `InputAxis|AimAzimuth`
  (params (AxisValue :type "Float (single-precision)"))
  (`SceneComponent.K2_AddLocalRotation` (`self.Azimuth Gimbal`) (`KismetMathLibrary.MakeRotator` 0.0 0.0 (* AxisValue (`GameplayStatics.GetWorldDeltaSeconds`) 100.0)) false false))

(event `InputAction|Fire`
  (params (Key :type "Key Structure"))
  (:`Pressed`
    (`self.Fire`)))

(event `InputAxis|Elevation`
  (params (AxisValue :type "Float (single-precision)"))
  (`SceneComponent.K2_AddLocalRotation` (`self.SpringArm`) (`KismetMathLibrary.MakeRotator` 0.0 (* AxisValue (`GameplayStatics.GetWorldDeltaSeconds`) 100.0)) false false))

(event `InputAxis|LeftTrack`
  (params (AxisValue :type "Float (single-precision)"))
  (`TankTrack.SetThrottle` (`self.LeftTrack`) AxisValue))

(event `InputAxis|ForwardMovement`
  (params (AxisValue :type "Float (single-precision)"))
  (`TankMovement.IntendMoveForward` (`self.TankMovement`) AxisValue))

(event `InputAxis|RightTrack`
  (params (AxisValue :type "Float (single-precision)"))
  (`TankTrack.SetThrottle` (`self.RightTrack`) AxisValue))

(event `InputAxis|RightMovement`
  (params (AxisValue :type "Float (single-precision)"))
  (`TankMovement.IntendMoveRight` (`self.TankMovement`) AxisValue))

(fn `UserConstructionScript`)